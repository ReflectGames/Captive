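; Barrel lid actor that locks onto or releases from a rain barrel through a physics constraint.
; Each tick it frees all linear and angular limits of the top's constraint once both the left and right lock parts are rotated past their yaw thresholds, printing a debug message.
; Otherwise, a short downward line trace from the lid re-locks every limit when it hits a component tagged RainBarrel.
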(event `self.ReceiveTick`
  (params (DeltaSeconds :type "Float (single-precision)"))
  (bind _top (`self.Top`))
  (bind _returnvalue (`SceneComponent.K2_GetComponentLocation` _top))
  (bind (_relativerotation_roll _relativerotation_pitch _relativerotation_yaw) (`KismetMathLibrary.BreakRotator` (`SceneComponent.RelativeRotation` (`self.RightLock`))))
  (bind (_relativerotation_roll_2 _relativerotation_pitch_2 _relativerotation_yaw_2) (`KismetMathLibrary.BreakRotator` (`SceneComponent.RelativeRotation` (`self.LeftLock`))))
  ;[1 1 1] Checks barrel lock progression
  (if (and (<= _relativerotation_yaw_2 -20.0) (<= _relativerotation_yaw -15.0))
    ;[1 1 1] Unlocks
    (`self.Unlocked`)
    (`KismetSystemLibrary.PrintString` "WE GUUD" true true (struct :`R` 0.133404 :`G` 1.0 :`A` 1.0) 0.0)
    (else
      ;[1 1 1] Checks if barrel lid is on then locks
      (bind (_outhit _returnvalue_2) (`KismetSystemLibrary.LineTraceSingle` _returnvalue (+ _returnvalue (* (`SceneComponent.GetUpVector` _top) -5.0)) "TraceTypeQuery1"))
      (if _returnvalue_2
        (if (`ActorComponent.ComponentHasTag` (`.HitComponent` (`GameplayStatics.BreakHitResult` _outhit)) "RainBarrel")
          (`self.Lock`))))))

(fn `Lock`
  (bind _top_physicsconstraint2 (`self.TOP PhysicsConstraint2`))
  (`PhysicsConstraintComponent.SetLinearXLimit` _top_physicsconstraint2 "LCM_Locked" 0.0)
  (`PhysicsConstraintComponent.SetLinearYLimit` _top_physicsconstraint2 "LCM_Locked" 0.0)
  (`PhysicsConstraintComponent.SetLinearZLimit` _top_physicsconstraint2 "LCM_Locked" 0.0)
  (`PhysicsConstraintComponent.SetAngularSwing1Limit` _top_physicsconstraint2 "ACM_Locked" 0.0)
  (`PhysicsConstraintComponent.SetAngularSwing2Limit` _top_physicsconstraint2 "ACM_Locked" 0.0)
  (`PhysicsConstraintComponent.SetAngularTwistLimit` _top_physicsconstraint2 "ACM_Locked" 0.0))

(fn `Unlocked`
  (bind _top_physicsconstraint2 (`self.TOP PhysicsConstraint2`))
  (`PhysicsConstraintComponent.SetLinearXLimit` _top_physicsconstraint2 "LCM_Free" 0.0)
  (`PhysicsConstraintComponent.SetLinearYLimit` _top_physicsconstraint2 "LCM_Free" 0.0)
  (`PhysicsConstraintComponent.SetLinearZLimit` _top_physicsconstraint2 "LCM_Free" 0.0)
  (`PhysicsConstraintComponent.SetAngularSwing1Limit` _top_physicsconstraint2 "ACM_Free" 0.0)
  (`PhysicsConstraintComponent.SetAngularSwing2Limit` _top_physicsconstraint2 "ACM_Free" 0.0)
  (`PhysicsConstraintComponent.SetAngularTwistLimit` _top_physicsconstraint2 "ACM_Free" 0.0))

(fn `UserConstructionScript`)